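; Berserker melee enemy that chases and damages the first-person player.
; Tick checks distance, turns the mesh toward the camera, runs AI MoveTo within attack range and sets MutantAnim detection and close-range flags.
; PlayerApplyDmg deals damage with a sound, while EnemyApplyDmg updates the health bar widget.
; At zero health it ragdolls, then after a delay calls the empty ItemRoulette stub and destroys itself.
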(event Custom|EnemyApplyDmg
  (params (DamageQty :type Float%20%28single-precision%29))
  ;[1 1 1] HealthManagement
  (bind _output_get (Variables|Default|SetCurrentHealth (- (Variables|Default|GetCurrentHealth) DamageQty)))
  (CallFunction|UpdateUIHealth)
  (if (<= _output_get 0.0)
    ;[1 1 1] OnDeath
    (CallFunction|EnableRagdoll)
    (Variables|Default|SetisDead true)
    (CallFunction|EnableRagdoll)
    (Utilities|FlowControl|Delay 3.0)
    (CallFunction|ItemRoulette)
    (Actor|DestroyActor)))

(event Custom|PlayerApplyDmg
  (if (not (Variables|Default|GetisDead))
    (bind _returnvalue (Actor|GetActorOfClass "/Game/MyStuff/Blueprints/FirstPersonCharacter.FirstPersonCharacter_C"))
    (Default|PlayerReceiveDamage _returnvalue (Variables|Default|GetDamage))
    (Audio|SpawnSoundatLocation "/Game/StarterContent/Audio/Collapse01.Collapse01" "0, 0, 0" "0, 0, 0" 0.35 1.0 0.0 0 0)))

(event EventBeginPlay)

(event Collision|EventActorBeginOverlap
  (params (OtherActor :type Actor%20Object%20Reference)))

(event EventTick
  (params (DeltaSeconds :type Float%20%28single-precision%29))
  (bind _mesh (Variables|Character|GetMesh))
  (bind _returnvalue (Components|SkeletalMesh|GetAnimInstance _mesh))
  (if (not (Variables|Default|GetisDead))
    ;[1 1 1] Player Perception
    (bind _returnvalue_2 (Actor|GetActorOfClass "/Game/MyStuff/Blueprints/FirstPersonCharacter.FirstPersonCharacter_C"))
    ;;[1 1 1] MoveTowards
    (bind _output_get (Variables|Default|SetCurrentDistance (Math|Vector|VectorLength (- (Transformation|GetActorLocation _returnvalue_2) (Transformation|GetActorLocation self)))))
    (bind _output_get_2 (Variables|Default|SetDetected (>= (Variables|Default|GetDetectRange) _output_get)))
    (if _output_get_2
      (CallFunction|UpdateLookPosition)
      (AI|AIMoveTo self (Transformation|GetActorLocation _returnvalue_2) 0 (Variables|Default|GetAttackRange) false
        (:then
          ;;[1 1 1] Detected Anim
          (bind _asmutant_anim (Utilities|Casting|CastToMutantAnim _returnvalue))
          (Variables|/Game/MyStuff/Models/Berserker/MutantAnim.MutantAnim_C|SetParam_Detected _asmutant_anim true))
        (:OnSuccess
          ;;[1 1 1] Attack
          ;;;[1 1 1] Attack Anim
          (bind _asmutant_anim_2 (Utilities|Casting|CastToMutantAnim _returnvalue))
          (Variables|/Game/MyStuff/Models/Berserker/MutantAnim.MutantAnim_C|SetParam_IsClose _asmutant_anim_2 true))
        (:OnFail
          (bind _asmutant_anim_3 (Utilities|Casting|CastToMutantAnim _returnvalue))
          (Variables|/Game/MyStuff/Models/Berserker/MutantAnim.MutantAnim_C|SetParam_IsClose _asmutant_anim_3 false)))
      (else
        (bind _asmutant_anim_4 (Utilities|Casting|CastToMutantAnim _returnvalue))
        (Variables|/Game/MyStuff/Models/Berserker/MutantAnim.MutantAnim_C|SetParam_Detected _asmutant_anim_4 false)))))

(fn ConstructionScript)

(fn EnableRagdoll
  (Class|SkeletalMeshComponent|SetAllBodiesSimulatePhysics (Variables|Character|GetMesh) true)
  (Collision|SetCollisionEnabled (Variables|Character|GetMesh) "PhysicsOnly")
  (Collision|SetCollisionEnabled (Variables|Collision|GetCapsuleComponent) "NoCollision"))

(fn SetAnimationDeath)

(fn UpdateUIHealth
  (bind _asui_health_bar (Utilities|Casting|CastToUI_HealthBar (UserInterface|GetWidget (Variables|Default|GetHealthBarContainer))))
  (Default|SetCurrentHealthUI _asui_health_bar (Variables|Default|GetCurrentHealth) 1e+02))

(fn GenerateAttackHitbox)

(fn UpdateLookPosition
  (bind _returnvalue (Game|GetPlayerCameraManager 0))
  (bind _mesh (Variables|Character|GetMesh))
  (bind _returnvalue_2 (Transformation|GetWorldLocation _mesh))
  (bind _returnvalue_3 (Camera|GetCameraLocation _returnvalue))
  (bind _returnvalue_4 (Math|Rotator|FindLookatRotation _returnvalue_2 _returnvalue_3))
  (bind (_roll _pitch _yaw) (Math|Rotator|BreakRotator _returnvalue_4))
  (Transformation|SetWorldRotation (Variables|Character|GetMesh) (Math|Rotator|MakeRotator _roll 0.0 (+ _yaw -9e+01)) false false))

(fn ItemRoulette)